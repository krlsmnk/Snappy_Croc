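; CoinToken is a coin token actor for VR that changes the player's hand pose when a hand comes near it.
; Begin overlap on HandAdjustRadius checks which Vive_PawnCharacter grab sphere entered, then gives that hand the pinch animation and switches its animation state.
; End overlap sets that hand to another animation state, without clearing the custom animation.
; The file contains no grab or pickup logic.
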(event OnComponentBeginOverlap(HandAdjustRadius)
  (params (OverlappedComponent :type Primitive%20Component%20Object%20Reference) (OtherActor :type Actor%20Object%20Reference) (OtherComp :type Primitive%20Component%20Object%20Reference) (OtherBodyIndex :type Integer) (bFromSweep :type Boolean) (SweepResult :type Hit%20Result%20Structure%20%28by%20ref%29))
  (bind _asvive_pawn_character (Utilities|Casting|CastToVive_PawnCharacter OtherActor))
  (Utilities|FlowControl|Sequence
    (:then_0
      (if (== (Variables|/Game/VRExpansion/Vive/Vive_PawnCharacter.Vive_PawnCharacter_C|GetGrabSphereRight _asvive_pawn_character) OtherComp)
        (Variables|/Game/VRExpansion/Vive/Testing/GraspingHand/GraspingHand.GraspingHand_C|SetCustomAnimation (Variables|/Game/VRExpansion/Vive/Vive_PawnCharacter.Vive_PawnCharacter_C|GetGraspingHandRight _asvive_pawn_character) "/Game/Blueprints/PinchAnim.PinchAnim")
        (Variables|/Game/VRExpansion/Vive/Testing/GraspingHand/GraspingHand.GraspingHand_C|SetHandAnimState (Variables|/Game/VRExpansion/Vive/Vive_PawnCharacter.Vive_PawnCharacter_C|GetGraspingHandRight _asvive_pawn_character) "NewEnumerator3")))
    (:then_1
      (if (== OtherComp (Variables|/Game/VRExpansion/Vive/Vive_PawnCharacter.Vive_PawnCharacter_C|GetGrabSphereLeft _asvive_pawn_character))
        (Variables|/Game/VRExpansion/Vive/Testing/GraspingHand/GraspingHand.GraspingHand_C|SetCustomAnimation (Variables|/Game/VRExpansion/Vive/Vive_PawnCharacter.Vive_PawnCharacter_C|GetGraspingHandLeft _asvive_pawn_character) "/Game/Blueprints/PinchAnim.PinchAnim")
        (Variables|/Game/VRExpansion/Vive/Testing/GraspingHand/GraspingHand.GraspingHand_C|SetHandAnimState (Variables|/Game/VRExpansion/Vive/Vive_PawnCharacter.Vive_PawnCharacter_C|GetGraspingHandLeft _asvive_pawn_character) "NewEnumerator3")))))

(event OnComponentEndOverlap(HandAdjustRadius)
  (params (OverlappedComponent :type Primitive%20Component%20Object%20Reference) (OtherActor :type Actor%20Object%20Reference) (OtherComp :type Primitive%20Component%20Object%20Reference) (OtherBodyIndex :type Integer))
  (bind _asvive_pawn_character (Utilities|Casting|CastToVive_PawnCharacter OtherActor))
  (Utilities|FlowControl|Sequence
    (:then_0
      (if (== (Variables|/Game/VRExpansion/Vive/Vive_PawnCharacter.Vive_PawnCharacter_C|GetGrabSphereRight _asvive_pawn_character) OtherComp)
        (Variables|/Game/VRExpansion/Vive/Testing/GraspingHand/GraspingHand.GraspingHand_C|SetHandAnimState (Variables|/Game/VRExpansion/Vive/Vive_PawnCharacter.Vive_PawnCharacter_C|GetGraspingHandRight _asvive_pawn_character) "NewEnumerator0")))
    (:then_1
      (if (== OtherComp (Variables|/Game/VRExpansion/Vive/Vive_PawnCharacter.Vive_PawnCharacter_C|GetGrabSphereLeft _asvive_pawn_character))
        (Variables|/Game/VRExpansion/Vive/Testing/GraspingHand/GraspingHand.GraspingHand_C|SetHandAnimState (Variables|/Game/VRExpansion/Vive/Vive_PawnCharacter.Vive_PawnCharacter_C|GetGraspingHandLeft _asvive_pawn_character) "NewEnumerator0")))))

(event EventBeginPlay)

(event Collision|EventActorBeginOverlap
  (params (OtherActor :type Actor%20Object%20Reference)))

(event EventTick
  (params (DeltaSeconds :type Float%20%28single-precision%29)))

(fn ConstructionScript)