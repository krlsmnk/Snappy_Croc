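; Game state for a Whack-A-Croc style arcade game, handling start, scoring, difficulty and graded end-of-game voice lines.
; After a delayed start it runs the AI controller's behavior tree and syncs phase to the blackboard, while Tick extends random crocs within delay and concurrency limits.
; PhaseSwitcher ramps difficulty using a PlayerSkill factor that bites lower, and Windup waits for full retraction before switching.
; Older timer-based phase logic is left unconnected.
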(event Custom|CheckTime
  ;[1 0 0] Phase Progression
)

(event Custom|End%20Game
  (bind _whacks (Variables|Default|GetWhacks))
  (bind _bites (Variables|Default|GetBites))
  (bind _possiblewhacks (Variables|Default|GetPossibleWhacks))
  (bind _returnvalue (Math|Conversions|ToFloat(Integer) _possiblewhacks))
  (bind _returnvalue_2 (* _bites 2))
  (bind _returnvalue_3 (- _whacks _returnvalue_2))
  (bind _returnvalue_4 (Math|Conversions|ToFloat(Integer) _returnvalue_3))
  (bind _returnvalue_5 (/ _returnvalue_4 _returnvalue))
  ;[1 1 1] End of Game Sequence
  (Actor|Tick|SetActorTickEnabled false)
  (Utilities|FlowControl|Delay 2.0)
  (if (> _returnvalue_3 (Variables|Default|GetHighScore)) ; New High Score?
    (Variables|Default|SetHighScore _returnvalue_3))
  (if (<= _returnvalue_5 0.29)
    (CallFunction|PlaySound "/Game/sound_effects/sfx/you_missed_me.you_missed_me")
    (CallFunction|SetResultEnum "NewEnumerator0")
    (Utilities|Time|SetTimerbyEvent (delegate Custom|MakeReady) 8.0 :!label _label)
    (elif (Math|Float|InRange(Float) _returnvalue_5 0.3 0.49)
      (CallFunction|PlaySound "/Game/sound_effects/sfx/try_harder.try_harder")
      (CallFunction|SetResultEnum "NewEnumerator1")
      (goto _label)
      (elif (Math|Float|InRange(Float) _returnvalue_5 0.5 0.69)
        (CallFunction|PlaySound "/Game/sound_effects/sfx/you_can_do_better.you_can_do_better")
        (CallFunction|SetResultEnum "NewEnumerator2")
        (goto _label)
        (elif (Math|Float|InRange(Float) _returnvalue_5 0.7 0.79)
          (CallFunction|PlaySound "/Game/sound_effects/sfx/pretty_good.pretty_good")
          (CallFunction|SetResultEnum "NewEnumerator3")
          (goto _label)
          (elif (>= _returnvalue_5 0.8)
            (CallFunction|PlaySound "/Game/sound_effects/sfx/you_win.you_win")
            (CallFunction|SetResultEnum "NewEnumerator4")
            (goto _label)))))))

(event Custom|Restart
  ;[1 1 1] Restart the Level
  (Development|ExecuteConsoleCommand "RestartLevel" 0))

(event Custom|Windup
  ;[1 1 1] Pause / Delay logic before final"speed phase"
  (Variables|Default|SetLockExtensions true)
  (Utilities|FlowControl|RetriggerableDelay 2.0) ; Keeps waiting until all retracted\nThen plays sound\nThen starts next phase
  (Variables|Default|SetCurrentDelay 1e+01) ; Delay the extension logic
  (if (== (Variables|Default|GetCurrentExtensions) 0) ; All retracted?
    (CallFunction|PlaySound "/Game/sound_effects/sfx/now_im_angry.now_im_angry")
    (Variables|Default|SetCurrentDelay 2.0)
    (CallFunction|PhaseSwitcher)
    (Variables|Default|SetLockExtensions false)
    (else
      (CallFunction|Windup) ; Recursive until all retracted
    )))

(event Custom|PhaseSwitcher
  (bind _maxsimultaneousextensions (Variables|Default|GetMaxSimultaneousExtensions))
  ;[0 1 1] Phase Changing Logic
  (bind _result (Math|Integer|IncrementInt (Variables|Default|GetCurrentPhase))
    (:%20%20
      (CallFunction|UpdateBlackBoardPhase)
      (if (>= (Variables|Default|GetPlayerSkill) 1.0) ; Is player good?
        (if (== (Math|Integer|%(Integer) (- _result 2) 3) 0) ; Every 3rd Phase:
          (if (< _maxsimultaneousextensions 3) ; If we can't do more...
            (Math|Integer|IncrementInt _maxsimultaneousextensions)
            (else
              (Variables|Default|SetExtensionSpeed (* (* (Variables|Default|GetExtensionSpeed) (Variables|Default|GetPlayerSkill)) 1.15)) ; Make them faster
            ))
          (else
            (Variables|Default|SetTimeBetweenExtensions (Math|Float|Clamp(Float) (* (/ (Variables|Default|GetTimeBetweenExtensions) (Variables|Default|GetPlayerSkill)) 0.75) 0.1 3.0))))))))

(event Custom|UpdateBlackBoardPhase
  (Class|BlackboardComponent|SetValueasInt (AI|GetBlackboard (stale Custom|Release%20the%20Crocs _returnvalue)) (Utilities|String|StringToName "Phase") (Variables|Default|GetCurrentPhase)))

(event Custom|StartGame
  (CallFunction|SetResultEnum "NewEnumerator6")
  (Variables|Default|SetWhacks 0)
  (Variables|Default|SetBites 0)
  (Variables|Default|SetPlayerSkill 1.0)
  (Variables|Default|SetCurrentPhase 1)
  (Variables|Default|SetExtensionSpeed 2e+01)
  (Variables|Default|SetCurrentExtensions 0)
  (Variables|Default|SetGameStatusResult "NewEnumerator6")
  (Variables|Default|SetMaxSimultaneousExtensions 1)
  (Variables|Default|SetLockExtensions false)
  (CallFunction|PlaySound "/Game/sound_effects/sfx/tokenAcceptCabinet.tokenAcceptCabinet")
  (Utilities|Time|SetTimerbyEvent (delegate Custom|Release%20the%20Crocs) 3.5))

(event Custom|Release%20the%20Crocs
  (Actor|Tick|SetActorTickEnabled true)
  ;[1 1 1] Begin Play Setup
  (CallFunction|PlaySound "/Game/sound_effects/sfx/im_gonna_get_you.im_gonna_get_you")
  (bind _returnvalue (Actor|GetActorOfClass "/Game/BP_CrocGameAIController.BP_CrocGameAIController_C"))
  (Utilities|FlowControl|Sequence
    (:then_0
      ;[1 0 0] Endless Mode Check
      (Utilities|IsValid (AI|GetBlackboard _returnvalue)
        (:Is%20Valid
          (AI|Components|Blackboard|SetValueasBool (AI|GetBlackboard _returnvalue) (Utilities|String|StringToName "EndlessMode") (Variables|Default|GetEndlessMode)) ; Tell AIController if on endless
        )))
    (:then_1
      (AI|RunBehaviorTree _returnvalue "/Game/CrocGame_BehaviorTree.CrocGame_BehaviorTree")
      (Class|BlackboardComponent|SetValueasInt (AI|GetBlackboard _returnvalue) (Utilities|String|StringToName "Phase") (Variables|Default|GetCurrentPhase)))))

(event Custom|MakeReady
  (CallFunction|SetResultEnum "NewEnumerator5") ; Allows coins to accept and restart
)

(event EventBeginPlay
  ;[1 1 1] Begin Play Setup
  (CallFunction|SetResultEnum "NewEnumerator5")
  (if (Utilities|Array|IsValidIndex (Variables|Default|GetCrocArray))
    (Variables|Default|SetCurrentDelay (Variables|Default|GetTimeBetweenExtensions))))

(event EventTick
  (params (DeltaSeconds :type Float%20%28single-precision%29))
  ;[1 1 1] Event Tick
  (Variables|Default|SetRemainingGameTime (- (Variables|Default|GetRemainingGameTime) DeltaSeconds)) ; Time remaining
  (Utilities|FlowControl|Sequence
    (:then_1
      (Variables|Default|SetCurrentDelay (- (Variables|Default|GetCurrentDelay) DeltaSeconds))
      (if (< (Variables|Default|GetCurrentExtensions) (Variables|Default|GetMaxSimultaneousExtensions)) ; Can we extend another?
        (if (<= (Variables|Default|GetCurrentDelay) 0.0) ; Delay time up?
          (bind _output (CallFunction|GetCrocbyIndex (Math|Random|RandomIntegerinRange 0 (- (Utilities|Array|Length (Variables|Default|GetCrocArray)) 1)))) ; Pick one randomly
          (if (Utilities|IsValid _output) ; check for null
            (if (not (Variables|Default|GetLockExtensions))
              (CallFunction|ExtensionCheck _output) ; Try to extend it
            )))
        (else
          (Variables|Default|SetCurrentDelay (Variables|Default|GetTimeBetweenExtensions)) ; delay extension logic
        )))))

(fn ConstructionScript
  (bind _outactors (Actor|GetAllActorsOfClass "/Game/Croc.Croc_C"))
  (if (Utilities|Array|IsValidIndex _outactors)
    (Variables|Default|SetCrocArray _outactors)
    (else
      (Development|PrintString "Empty"))))

(fn ExtensionCheck
  (params (WhichCroc :type Croc%20Object%20Reference))
  (Variables|Default|SetCurrentCroc WhichCroc)
  (if (< (Variables|Default|GetCurrentExtensions) (Variables|Default|GetMaxSimultaneousExtensions)) ; Can we extend another?
    (if (Variables|/Game/Croc.Croc_C|GetExtended (Variables|Default|GetCurrentCroc)) ; If target croc already extended
      (bind _output (CallFunction|GetCrocbyIndex (+ (Variables|/Game/Croc.Croc_C|GetIndex (Variables|Default|GetCurrentCroc)) 1))) ; Get the "next" one and try it
      (if (not (== _output (Variables|Default|GetCurrentCroc))) ; Prevents infinite edge case for 1 croc
        (CallFunction|ExtensionCheck _output))
      (else
        (Default|PerformExtension (Variables|Default|GetCurrentCroc))))))

(fn GetCrocbyIndex
  (params (Index :type Integer))
  (bind _crocarray (Variables|Default|GetCrocArray))
  (if (<= Index (Utilities|Array|Length _crocarray)) ; IS requested index within Bounds?
    (return (Utilities|Array|Get(acopy) _crocarray Index))
    (else
      (return (Utilities|Array|Get(acopy) (Variables|Default|GetCrocArray))))))

(fn Bite
  (Math|Integer|IncrementInt (Variables|Default|GetBites)
    (:%20%20
      (Variables|Default|SetPlayerSkill (* (Variables|Default|GetPlayerSkill) 0.85)) ; Skill penalty to reduce difficulty
      (switch int (Math|Random|RandomIntegerinRange 0 3)
        (:Default
          (Audio|Components|Audio|Play (Variables|Default|GetBiteSound) 0.0 :!label _label))
        (:0
          (CallFunction|PlaySound "/Game/sound_effects/sfx/crunch.crunch"))
        (:1
          (CallFunction|PlaySound "/Game/sound_effects/sfx/crunch_2.crunch_2"))
        (:2
          (CallFunction|PlaySound "/Game/sound_effects/sfx/crunch_3.crunch_3"))
        (:3
          (goto _label))))))

(fn PlaySound
  (params (SoundToPlay :type Sound%20Wave%20Object%20Reference))
  (bind _genericsoundplayer (Variables|Default|GetGenericSoundPlayer))
  (Audio|Components|Audio|SetSound _genericsoundplayer SoundToPlay)
  (Audio|Components|Audio|Play _genericsoundplayer 0.0))

(fn SetResultEnum
  (params (State :type GameStateResult%20Enum :default "NewEnumerator0"))
  (bind _output_get (Variables|Default|SetGameStatusResult State))
  (Default|CallResultEnumUpdater _output_get))