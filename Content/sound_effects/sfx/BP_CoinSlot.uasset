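; BP_CoinSlot is a coin slot trigger that starts the Croc game when a coin or token is inserted.
; Its box overlap event acts only while the Croc game state reports the stopped status.
; It recognizes coins by searching the overlapping actor's display name for "token" or "coin", then destroys the actor and calls StartGame on the game state.
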(event OnComponentBeginOverlap(OverlapBox)
  (params (OverlappedComponent :type Primitive%20Component%20Object%20Reference) (OtherActor :type Actor%20Object%20Reference) (OtherComp :type Primitive%20Component%20Object%20Reference) (OtherBodyIndex :type Integer) (bFromSweep :type Boolean) (SweepResult :type Hit%20Result%20Structure%20%28by%20ref%29))
  (bind _returnvalue (Utilities|GetDisplayName OtherActor))
  (bind _ascroc_game_state (Utilities|Casting|CastToCrocGameState (Game|GetGameState)))
  (if (Utilities|Enum|Equal(Enum) (Variables|/Game/Blueprints/CrocGameState.CrocGameState_C|GetGameStatusResult _ascroc_game_state) "NewEnumerator5") ; only accept coin if game stopped
    (Utilities|IsValid OtherActor
      (:Is%20Valid
        (if (or (Utilities|String|Contains _returnvalue "token") (Utilities|String|Contains _returnvalue "coin")) ; Is it the coin?
          (Actor|DestroyActor OtherActor) ; Take coin
          (bind _ascroc_game_state_2 (Utilities|Casting|CastToCrocGameState (Game|GetGameState)))
          (Default|StartGame _ascroc_game_state_2))))))

(event EventBeginPlay)

(event Collision|EventActorBeginOverlap
  (params (OtherActor :type Actor%20Object%20Reference)))

(event EventTick
  (params (DeltaSeconds :type Float%20%28single-precision%29)))

(fn ConstructionScript)